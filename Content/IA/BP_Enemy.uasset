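; BP_Enemy is an enemy Blueprint that can hurt the player in melee range.
; AttackEvent checks whether the AttackBOx overlaps the player pawn, then casts it to BP_ThirdPersonCharacter and calls its Dano function with a fixed damage amount.
; Its own Dano and Restore functions are empty, with disconnected health arithmetic and progress bar nodes.
; Damage and Regen only call those empty functions with zero, so neither changes health.
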(event `AttackEvent`
  (bind _returnvalue (`GameplayStatics.GetPlayerPawn` 0))
  (if (`PrimitiveComponent.IsOverlappingActor` (`self.AttackBOx`) _returnvalue)
    (bind _asbp_third_person_character (cast `/Game/ThirdPerson/Blueprints/BP_ThirdPersonCharacter` _returnvalue))
    (`/Game/ThirdPerson/Blueprints/BP_ThirdPersonCharacter.Dano` _asbp_third_person_character 5.0)))

(fn `Damage`
  (`self.Dano` 0.0))

(fn `Dano`
  (params (Damage :type "Float (double-precision)")))

(fn `Regen`
  (locals (NewLocalVar :type "Float (double-precision)"))
  (`self.restore` 0.0))

(fn `restore`
  (params (Damage :type "Float (double-precision)")))

(fn `UserConstructionScript`)