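; Key pickup actor that unlocks a linked Door by setting its HasKey flag when the player collects it.
; Box overlap toggles interactability and the player's look-at toward the key, and registers it as LastInteractObject.
; Interact sets the player's Pressed flag, waits, then destroys the key, whose Destroyed event updates an inventory HUD icon.
; A zero-delay loop from BeginPlay spins the mesh if CanRotate is initially true.
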(event `self.Box.OnComponentBeginOverlap`
  (params (OverlappedComponent :type "PrimitiveComponent Object Reference") (OtherActor :type "Actor Object Reference") (OtherComp :type "PrimitiveComponent Object Reference") (OtherBodyIndex :type Integer) (bFromSweep :type Boolean) (SweepResult :type "HitResult Structure (by ref)"))
  (bind _as_bp_third_person_character_player (`self.As BP Third Person Character Player`))
  ; CanInteract
  (bind _asbp_third_person_character_player (cast `/Game/BluePrint/CoreGameplay/BP_ThirdPersonCharacter_Player` OtherActor))
  (bind _output_get (set `self.As BP Third Person Character Player` _asbp_third_person_character_player))
  (set `/Game/BluePrint/CoreGameplay/BP_ThirdPersonCharacter_Player.LastInteractObject` self _output_get)
  (set `self.canInteract?` true)
  ; lookAt
  (set `/Game/BluePrint/CoreGameplay/BP_ThirdPersonCharacter_Player.LookAt_0` true _as_bp_third_person_character_player)
  (set `/Game/BluePrint/CoreGameplay/BP_ThirdPersonCharacter_Player.LookAtPosition_0` (`self.K2_GetActorLocation`) _as_bp_third_person_character_player))

(event `self.ReceiveDestroyed`
  (`Image.SetBrushFromTexture` (`/Game/BluePrint/Hud/Inventory_HUD.icon1` (`/Game/BluePrint/CoreGameplay/BP_ThirdPersonCharacter_Player.InventoryHud` (`self.As BP Third Person Character Player`))) "/Engine/EditorResources/Ai_Spawnpoint.Ai_Spawnpoint" false))

(event `self.ReceiveBeginPlay`
  ; RotateSettings
  (if (`self.CanRotate`)
    (`SceneComponent.K2_AddRelativeRotation` (`self.StaticMesh`) (struct :`Yaw` 1.0) false false :!label _label)
    (`KismetSystemLibrary.Delay` 0.0)
    (goto _label)))

(event `self.Box.OnComponentEndOverlap`
  (params (OverlappedComponent :type "PrimitiveComponent Object Reference") (OtherActor :type "Actor Object Reference") (OtherComp :type "PrimitiveComponent Object Reference") (OtherBodyIndex :type Integer))
  ; CanInteract
  (cast `/Game/BluePrint/CoreGameplay/BP_ThirdPersonCharacter_Player` OtherActor)
  (set `self.canInteract?` false)
  ; lookAt
  (set `/Game/BluePrint/CoreGameplay/BP_ThirdPersonCharacter_Player.LookAt_0` false (`self.As BP Third Person Character Player`)))

(event `/Game/BluePrint/interact.Interact`
  (bind _as_bp_third_person_character_player (`self.As BP Third Person Character Player`))
  ; Interact
  (if (`self.canInteract?`)
    (set `self.CanRotate` true)
    (set `/Game/BluePrint/CoreGameplay/BP_ThirdPersonCharacter_Player.Pressed?` true _as_bp_third_person_character_player)
    (set `/Game/BluePrint/CoreGameplay/BP_ThirdPersonCharacter_Player.LookAt_0` false _as_bp_third_person_character_player)
    (`KismetSystemLibrary.Delay` 5.0)
    (`/Engine/EditorBlueprintResources/StandardMacros.IsValid` (`self.StaticMesh`)
      (:`Is Valid`
        (`self.K2_DestroyActor`)
        (set `/Game/BluePrint/Door.HasKey?` true (`self.Door`))
        (set `/Game/BluePrint/CoreGameplay/BP_ThirdPersonCharacter_Player.Pressed?` false _as_bp_third_person_character_player)))))

(fn `UserConstructionScript`)