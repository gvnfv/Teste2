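; An interactable pickup item whose static mesh is set from its Item data at construction.
; Box overlap registers it as the player character's last interact object and turns on the player's look-at toward it, while leaving clears the interact flag and look-at.
; Interact passes the data table row name to the player's AddItem through the Body event, then destroys the actor.
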(event `self.Box.OnComponentBeginOverlap`
  (params (OverlappedComponent :type "PrimitiveComponent Object Reference") (OtherActor :type "Actor Object Reference") (OtherComp :type "PrimitiveComponent Object Reference") (OtherBodyIndex :type Integer) (bFromSweep :type Boolean) (SweepResult :type "HitResult Structure (by ref)"))
  (bind _as_bp_third_person_character_player (`self.As BP Third Person Character Player`))
  ; CanInteract
  (bind _asbp_third_person_character_player (cast `/Game/BluePrint/CoreGameplay/BP_ThirdPersonCharacter_Player` OtherActor))
  (bind _output_get (set `self.As BP Third Person Character Player` _asbp_third_person_character_player))
  (set `/Game/BluePrint/CoreGameplay/BP_ThirdPersonCharacter_Player.LastInteractObject` self _output_get)
  (set `self.CanInteract` true)
  ; lookAt
  (set `/Game/BluePrint/CoreGameplay/BP_ThirdPersonCharacter_Player.LookAt_0` true _as_bp_third_person_character_player)
  (set `/Game/BluePrint/CoreGameplay/BP_ThirdPersonCharacter_Player.LookAtPosition_0` (`self.K2_GetActorLocation`) _as_bp_third_person_character_player))

(event `/Game/BluePrint/interact.Interact`
  (`self.Body`)
  (`self.K2_DestroyActor`))

(event `self.Box.OnComponentEndOverlap`
  (params (OverlappedComponent :type "PrimitiveComponent Object Reference") (OtherActor :type "Actor Object Reference") (OtherComp :type "PrimitiveComponent Object Reference") (OtherBodyIndex :type Integer))
  ; CanInteract
  (cast `/Game/BluePrint/CoreGameplay/BP_ThirdPersonCharacter_Player` OtherActor)
  (set `self.CanInteract` false)
  ; lookAt
  (set `/Game/BluePrint/CoreGameplay/BP_ThirdPersonCharacter_Player.LookAt_0` false (`self.As BP Third Person Character Player`)))

(event `self.ReceiveDestroyed`)

(event `Body`
  (`/Game/BluePrint/CoreGameplay/BP_ThirdPersonCharacter_Player.AddItem` (`self.As BP Third Person Character Player`) (`.RowName` (break `DataTableRowHandle` (`self.DataTableRowHandle`)))))

(fn `UserConstructionScript`
  (`StaticMeshComponent.SetStaticMesh` (`self.StaticMesh`) (`.Mesh_11_36D10488474FDF391819B2825CAA57E3` (break `/Game/BluePrint/GameDesign/S_Items` (`self.Item`)))))