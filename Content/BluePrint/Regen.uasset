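; Regen is a healing zone that restores life to a BP_MasterCharacter standing inside its Box trigger.
; On overlap, if Life is below 100, it calls Dano with negative damage in a short-delay loop.
; The loop runs until end overlap clears a shared in-range flag, without rechecking Life between ticks.
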(event `self.Box.OnComponentBeginOverlap`
  (params (OverlappedComponent :type "PrimitiveComponent Object Reference") (OtherActor :type "Actor Object Reference") (OtherComp :type "PrimitiveComponent Object Reference") (OtherBodyIndex :type Integer) (bFromSweep :type Boolean) (SweepResult :type "HitResult Structure (by ref)"))
  (bind _asbp_master_character (cast `/Game/BluePrint/CoreGameplay/BP_MasterCharacter` OtherActor))
  (set `self.ItsInTheRange?` true)
  (if (< (`.Life_3_C74511DF4827D6961E14DE9C12EA3D6C` (break `/Game/BluePrint/GameDesign/S_Stats` (`/Game/BluePrint/CoreGameplay/BP_MasterCharacter.Stats` _asbp_master_character))) 100.0)
    (`/Game/BluePrint/CoreGameplay/BP_MasterCharacter.Dano` _asbp_master_character -1.0 :!label _label)
    (if (`self.ItsInTheRange?`)
      (`KismetSystemLibrary.Delay` 0.1)
      (goto _label))))

(event `self.Box.OnComponentEndOverlap`
  (params (OverlappedComponent :type "PrimitiveComponent Object Reference") (OtherActor :type "Actor Object Reference") (OtherComp :type "PrimitiveComponent Object Reference") (OtherBodyIndex :type Integer))
  (cast `/Game/BluePrint/CoreGameplay/BP_MasterCharacter` OtherActor)
  (set `self.ItsInTheRange?` false))

(fn `UserConstructionScript`)