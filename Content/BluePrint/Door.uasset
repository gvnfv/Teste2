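; Interactable hinged door that the player can open and close when its HasKey flag is set.
; A Box overlap registers the door as the player's LastInteractObject, enables interaction and shows the PressE prompt.
; Interact uses a FlipFlop to play or reverse the DoorT timeline, which drives the door's yaw.
; Timeline updates pulse the player's OpeningDoor and ClosingDoor flags for animation, based on Dooropen, which is set on finish.
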(event `/Game/BluePrint/interact.Interact`
  (bind _as_bp_third_person_character_player (`self.As BP Third Person Character Player`))
  (if (`self.HasKey?`)
    (if (`self.CanInteract?`)
      (`Widget.RemoveFromParent` (`/Game/BluePrint/CoreGameplay/BP_ThirdPersonCharacter_Player.pressE` (`self.As BP Third Person Character Player`)))
      (`/Engine/EditorBlueprintResources/StandardMacros.FlipFlop`
        (:`A`
          (bind (_direction _doorm) (`Timeline|DoorT` :!label _label)
            (:`Update`
              (`SceneComponent.K2_SetRelativeRotation` (`self.Door`) (`KismetMathLibrary.MakeRotator` 0.0 0.0 _doorm) false false)
              (`|ExecutionSequence`
                (:`then_0`
                  ; Animation_open/close
                  (set `/Game/BluePrint/CoreGameplay/BP_ThirdPersonCharacter_Player.ClosingDoor` (`self.Dooropen?`) _as_bp_third_person_character_player)
                  (`KismetSystemLibrary.Delay` 2.0)
                  (set `/Game/BluePrint/CoreGameplay/BP_ThirdPersonCharacter_Player.ClosingDoor` false _as_bp_third_person_character_player))
                (:`then_1`
                  (set `/Game/BluePrint/CoreGameplay/BP_ThirdPersonCharacter_Player.OpeningDoor` (not (`self.Dooropen?`)) _as_bp_third_person_character_player)
                  (`KismetSystemLibrary.Delay` 2.0)
                  (set `/Game/BluePrint/CoreGameplay/BP_ThirdPersonCharacter_Player.OpeningDoor` false _as_bp_third_person_character_player))))
            (:`Finished`
              (set `self.Dooropen?` (> _doorm 0.0)))))
        (:`B`
          (if (`self.Dooropen?`)
            (goto _label :!via `Reverse`)))))))

(event `self.Box.OnComponentBeginOverlap`
  (params (OverlappedComponent :type "PrimitiveComponent Object Reference") (OtherActor :type "Actor Object Reference") (OtherComp :type "PrimitiveComponent Object Reference") (OtherBodyIndex :type Integer) (bFromSweep :type Boolean) (SweepResult :type "HitResult Structure (by ref)"))
  (bind _asbp_third_person_character_player (cast `/Game/BluePrint/CoreGameplay/BP_ThirdPersonCharacter_Player` OtherActor))
  (bind _output_get (set `self.As BP Third Person Character Player` _asbp_third_person_character_player))
  (set `/Game/BluePrint/CoreGameplay/BP_ThirdPersonCharacter_Player.LastInteractObject` self _output_get)
  (set `self.CanInteract?` true)
  (`UserWidget.AddToViewport` (`/Game/BluePrint/CoreGameplay/BP_ThirdPersonCharacter_Player.pressE` _output_get) 0))

(event `self.Box.OnComponentEndOverlap`
  (params (OverlappedComponent :type "PrimitiveComponent Object Reference") (OtherActor :type "Actor Object Reference") (OtherComp :type "PrimitiveComponent Object Reference") (OtherBodyIndex :type Integer))
  (cast `/Game/BluePrint/CoreGameplay/BP_ThirdPersonCharacter_Player` OtherActor)
  (set `self.CanInteract?` false)
  (`Widget.RemoveFromParent` (`/Game/BluePrint/CoreGameplay/BP_ThirdPersonCharacter_Player.pressE` (stale `self.Box.OnComponentBeginOverlap` _output_get))))

(fn `UserConstructionScript`)