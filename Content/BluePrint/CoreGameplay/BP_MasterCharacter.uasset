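; BP_MasterCharacter is a master character Blueprint providing melee-style damage and health for player and enemy characters.
; Construction loads Life into Stats from the Enemy01 row of DT_Charbalance.
; CollisionAttack overlaps store an opposing target, with IsPlayer choosing the enemy or player cast, and clear it on exit.
; Attack calls Dano on that target, which subtracts Life, prints debug text and destroys the actor below zero.
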(event `self.collisionAttack.OnComponentBeginOverlap`
  (params (OverlappedComponent :type "PrimitiveComponent Object Reference") (OtherActor :type "Actor Object Reference") (OtherComp :type "PrimitiveComponent Object Reference") (OtherBodyIndex :type Integer) (bFromSweep :type Boolean) (SweepResult :type "HitResult Structure (by ref)"))
  (if (`self.IsPlayer`)
    (bind _asbp_enemy_master (cast `/Game/BluePrint/CoreGameplay/BP_EnemyMaster` OtherActor))
    (set `self.OtherActor` _asbp_enemy_master)
    (else
      (bind _asbp_third_person_character_player (cast `/Game/BluePrint/CoreGameplay/BP_ThirdPersonCharacter_Player` OtherActor))
      (set `self.OtherActor` _asbp_third_person_character_player))))

(event `self.collisionAttack.OnComponentEndOverlap`
  (params (OverlappedComponent :type "PrimitiveComponent Object Reference") (OtherActor :type "Actor Object Reference") (OtherComp :type "PrimitiveComponent Object Reference") (OtherBodyIndex :type Integer))
  (if (== OtherActor (`self.OtherActor`))
    (set `self.OtherActor` null)))

(fn `Attack`
  (params (amount :type "Float (double-precision)"))
  (bind _otheractor (`self.OtherActor`))
  (`KismetSystemLibrary.PrintString` "attack")
  (`/Engine/EditorBlueprintResources/StandardMacros.IsValid` _otheractor
    (:`Is Valid`
      (`self.Dano` _otheractor amount))))

(fn `Dano`
  (params (Much :type "Float (double-precision)"))
  (locals (NewLocalVar :type "Float (double-precision)"))
  (bind _stats (`self.Stats`))
  (bind _returnvalue (- (`.Life_3_C74511DF4827D6961E14DE9C12EA3D6C` (break `/Game/BluePrint/GameDesign/S_Stats` _stats)) Much))
  (setmembers `/Game/BluePrint/GameDesign/S_Stats` :`StructRef` _stats :`Life` _returnvalue)
  (if (< _returnvalue 0.0)
    (`KismetSystemLibrary.PrintString` "Dead")
    (`self.K2_DestroyActor`)
    (else
      (`KismetSystemLibrary.PrintString` (`KismetStringLibrary.Conv_DoubleToString` _returnvalue)))))

(fn `UserConstructionScript`
  (bind _returnvalue (`|GetDataTableRow` "/Game/BluePrint/GameDesign/DT_Charbalance.DT_Charbalance" "Enemy01")
    (:`then`
      (setmembers `/Game/BluePrint/GameDesign/S_Stats` :`StructRef` (`self.Stats`) :`Life` (`.Life_6_475E427C4F303E7C218745AC9E4E9CE7` (break `/Game/BluePrint/GameDesign/S_EnemyBalance` _returnvalue))))))