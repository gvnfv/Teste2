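; Base enemy Blueprint that takes its balance values from a data table and triggers attacks.
; Its construction script runs the parent's, then reads the hardcoded Enemy01 row of DT_Charbalance into Life, ReactionTime and SightDistance.
; It also writes the reaction time to the AI controller's Blackboard Reaction key during construction.
; The AttackNoti event calls Attack with a fixed value, independent of the table.
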(event `AttackNoti`
  (`self.Attack` 10.0))

(fn `UserConstructionScript`
  (`parent.UserConstructionScript`)
  (bind _returnvalue (`|GetDataTableRow` "/Game/BluePrint/GameDesign/DT_Charbalance.DT_Charbalance" "Enemy01")
    (:`then`
      (bind (_life _sightdistance _reactiontime) (break `/Game/BluePrint/GameDesign/S_EnemyBalance` _returnvalue))
      (setmembers `/Game/BluePrint/GameDesign/S_Stats` :`StructRef` (`self.Stats`) :`Life` _life)
      (bind _output_get (set `self.Reaction Time` _reactiontime))
      (set `self.Sight Distance` _sightdistance)
      (`BlackboardComponent.SetValueAsFloat` (`AIController.Blackboard` (`AIBlueprintHelperLibrary.GetAIController` null)) "Reaction" _output_get))))